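; Player controller that links the player character and game instance to the HUD and switches between gameplay and UI-only input.
; Character pickup and combinable-overlap events drive item info and messages, while input actions show hints and an exit prompt.
; On BeginPlay it frees the cursor if the tutorial is unseen, or shows the end-game view once all levels are passed.
; ResetProgress clears passed-level checks and opens scenario selection.
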(event Custom|Event%20BeginCombinableOverlap
  (params (CombinableKind :type BPE_CombinableItems%20Enum :default "NewEnumerator0"))
  (CallFunction|TryShowCombinableMessage CombinableKind))

(event Custom|Event%20ItemPickedUp
  (params (Item :type BP%20Holdable%20Item%20Object%20Reference))
  (Default|SetItemValuesView (Variables|/Game/TestTask/Blueprints/Ui/BP_HUD.BP_HUD_C|GetItemsInfo (Variables|Default|GetHud)) Item true))

(event Custom|Event%20ItemReleased
  (Default|SetItemValuesView (Variables|/Game/TestTask/Blueprints/Ui/BP_HUD.BP_HUD_C|GetItemsInfo (Variables|Default|GetHud)) 0 false))

(event Custom|Event%20EndCombinableOverlap
  (Default|SetCombinableItemMessage (Variables|/Game/TestTask/Blueprints/Ui/BP_HUD.BP_HUD_C|GetItemsInfo (Variables|Default|GetHud)) 0 false))

(event EventBeginPlay
  (bind _asbp_player_character (Utilities|Casting|CastToBP_PlayerCharacter (Game|GetPlayerCharacter 0)))
  (Variables|Default|SetPlayerCharacter _asbp_player_character)
  (bind _asbp_hud (Utilities|Casting|CastToBP_HUD (HUD|GetHUD)))
  (Variables|Default|SetHud _asbp_hud)
  (bind _asbp_game_instance (Utilities|Casting|CastToBP_GameInstance (Game|GetGameInstance)))
  (Variables|Default|SetGameInstance _asbp_game_instance)
  (Utilities|FlowControl|Sequence
    (:then_0
      (CallFunction|SetInput (Math|Boolean|NotEqual(Boolean) (Variables|/Game/TestTask/Blueprints/BP_GameInstance.BP_GameInstance_C|GetTutorialIsShown (Variables|Default|GetGameInstance)) true))
      (if (CallFunction|CanEndGame)
        (Utilities|FlowControl|Delay 0.5)
        (Widget|SetVisibility (Variables|/Game/TestTask/Blueprints/Ui/BP_HUD.BP_HUD_C|GetEndGameView (Variables|Default|GetHud)) "Visible")
        (CallFunction|SetInput true)
        (Default|SetQuestsChecks (Variables|/Game/TestTask/Blueprints/Ui/BP_HUD.BP_HUD_C|GetEndGameView (Variables|Default|GetHud)))))
    (:then_1
      (EventDispatchers|BindEventtoItemPickedUp (Variables|Default|GetPlayerCharacter) (delegate Custom|Event%20ItemPickedUp))
      (EventDispatchers|BindEventtoItemReleased (Variables|Default|GetPlayerCharacter) (delegate Custom|Event%20ItemReleased)))
    (:then_2
      (EventDispatchers|BindEventtoOnBeginOverlapCombinable (Variables|Default|GetPlayerCharacter) (delegate Custom|Event%20BeginCombinableOverlap))
      (EventDispatchers|BindEventtoOnEndOverlapCombinable (Variables|Default|GetPlayerCharacter) (delegate Custom|Event%20EndCombinableOverlap)))))

(event Input|ActionEvents|InputActionShowHint
  (params (Key :type Key%20Structure :default "None"))
  (bind _hud (Variables|Default|GetHud))
  (bind _hints (Variables|/Game/TestTask/Blueprints/Ui/BP_HUD.BP_HUD_C|GetHints _hud))
  (:Pressed
    (if (not (< (Variables|/Game/TestTask/Blueprints/BP_GameInstance.BP_GameInstance_C|GetCurrentLevelId (Variables|Default|GetGameInstance)) 0))
      (Widget|SetVisibility _hints "Visible")
      (CallFunction|SetInput false)))
  (:Released
    (Widget|SetVisibility _hints "Hidden")
    (CallFunction|SetInput false)))

(event Input|ActionEvents|InputActionExitGame
  (params (Key :type Key%20Structure :default "None"))
  (:Pressed
    (if (Variables|/Game/TestTask/Blueprints/BP_GameInstance.BP_GameInstance_C|GetTutorialIsShown (Variables|Default|GetGameInstance))
      (CallFunction|SetInput true)
      (Widget|SetVisibility (Variables|/Game/TestTask/Blueprints/Ui/BP_HUD.BP_HUD_C|GetExitMessage (Variables|Default|GetHud)) "Visible"))))

(fn ConstructionScript)

(fn TryShowCombinableMessage
  (params (CombinableKind :type BPE_CombinableItems%20Enum :default "NewEnumerator0"))
  (if (Utilities|Enum|NotEqual(Enum) CombinableKind "NewEnumerator1")
    (Default|SetCombinableItemMessage (Variables|/Game/TestTask/Blueprints/Ui/BP_HUD.BP_HUD_C|GetItemsInfo (Variables|Default|GetHud)) 0 true)))

(fn SetInput
  (params (IsShow :type Boolean))
  (bind _self self)
  (bind _self_2 self)
  (if IsShow
    (Input|DisableInput _self)
    (Variables|Default|SetbShowMouseCursor true)
    (Input|SetInputModeUIOnly _self_2 0 "DoNotLock")
    (else
      (Input|EnableInput _self)
      (Variables|Default|SetbShowMouseCursor false)
      (Input|SetInputModeGameOnly _self_2))))

(fn ResetProgress
  (bind _gameinstance (Variables|Default|GetGameInstance))
  (bind _passedlevelschecks (Variables|/Game/TestTask/Blueprints/BP_GameInstance.BP_GameInstance_C|GetPassedLevelsChecks _gameinstance))
  (for (_ _array_index) _passedlevelschecks
    (Utilities|Array|SetArrayElem _passedlevelschecks _array_index false))
  (Game|OpenLevel(byObjectReference) "/Game/TestTask/Maps/ScenarioSelectionMap.ScenarioSelectionMap"))

(fn CanEndGame
  (for _array_element (Variables|/Game/TestTask/Blueprints/BP_GameInstance.BP_GameInstance_C|GetPassedLevelsChecks (Variables|Default|GetGameInstance))
    (if (not _array_element)
      (return false)))
  (return true))