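; First-person player character that moves, looks, and can hold, use, release and combine one item at a time.
; A camera line trace sends interact messages and attaches free holdable items to a holding point.
; While holding, capsule overlaps track the current combinable via interface messages, enabling combining on input or triggering it immediately for one kind.
; Event dispatchers broadcast pickup, release and combinable overlap changes, with pickup re-broadcast when an item action ends.
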(event OnComponentBeginOverlap(CapsuleComponent)
  (params (OverlappedComponent :type Primitive%20Component%20Object%20Reference) (OtherActor :type Actor%20Object%20Reference) (OtherComp :type Primitive%20Component%20Object%20Reference) (OtherBodyIndex :type Integer) (bFromSweep :type Boolean) (SweepResult :type Hit%20Result%20Structure%20%28by%20ref%29))
  (if (Variables|Default|GetIsBusy)
    (bind _output_get (Variables|Default|SetCurrentCombinable OtherActor))
    (bind (_kind _isbusy) (Class|BPICombinable|GetKind(Message) _output_get))
    (if (not _isbusy)
      (Default|CallOnBeginOverlapCombinable _kind)
      (Variables|Default|SetCanCombineItems true)
      (if (Utilities|Enum|Equal(Enum) _kind "NewEnumerator1")
        (Class|BPICombinable|TryCombine(Message) (Variables|Default|GetCurrentCombinable) (Variables|Default|GetHoldedItem))))))

(event OnComponentEndOverlap(CapsuleComponent)
  (params (OverlappedComponent :type Primitive%20Component%20Object%20Reference) (OtherActor :type Actor%20Object%20Reference) (OtherComp :type Primitive%20Component%20Object%20Reference) (OtherBodyIndex :type Integer))
  (Utilities|Casting|CastToBPI_Combinable OtherActor)
  (Default|CallOnEndOverlapCombinable)
  (Variables|Default|SetCanCombineItems false))

(event Input|ActionEvents|InputActionCombineAction
  (params (Key :type Key%20Structure :default "None"))
  (:Pressed
    (if (and (Variables|Default|GetIsBusy) (Variables|Default|GetCanCombineItems))
      (Class|BPICombinable|TryCombine(Message) (Variables|Default|GetCurrentCombinable) (Variables|Default|GetHoldedItem)))))

(event Input|ActionEvents|InputActionDoAction
  (params (Key :type Key%20Structure :default "None"))
  (:Pressed
    (if (Variables|Default|GetIsBusy)
      (CallFunction|ReleaseItem)
      (else
        (CallFunction|TryInteract)))))

(event Input|ActionEvents|InputActionItemAction
  (params (Key :type Key%20Structure :default "None"))
  (:Pressed
    (if (Variables|Default|GetIsBusy)
      (Class|BPIActionable|DoAction(Message) (Variables|Default|GetHoldedItem)))))

(event Input|AxisEvents|InputAxisMoveHorizontal
  (params (AxisValue :type Float%20%28single-precision%29))
  (Pawn|Input|AddMovementInput (Transformation|GetActorRightVector) AxisValue false))

(event Input|AxisEvents|InputAxisMoveVertical
  (params (AxisValue :type Float%20%28single-precision%29))
  (Pawn|Input|AddMovementInput (Transformation|GetActorForwardVector) AxisValue false))

(event Input|AxisEvents|InputAxisLookHorizontal
  (params (AxisValue :type Float%20%28single-precision%29))
  (Pawn|Input|AddControllerYawInput AxisValue))

(event Input|AxisEvents|InputAxisLookVertical
  (params (AxisValue :type Float%20%28single-precision%29))
  (Pawn|Input|AddControllerPitchInput AxisValue))

(fn ConstructionScript)

(fn PickUpItem
  (params (HoldableItem :type BP%20Holdable%20Item%20Object%20Reference))
  (bind _output_get (Variables|Default|SetHoldedItem HoldableItem))
  (Transformation|AttachComponentToComponent _output_get (Variables|Default|GetHoldingPoint) "None" "SnapToTarget" "SnapToTarget" "KeepRelative" true)
  (Variables|Default|SetIsBusy true)
  (Default|CallItemPickedUp (Variables|Default|GetHoldedItem))
  (EventDispatchers|BindEventtoActionEnded (Variables|Default|GetHoldedItem) (EventDispatchers|CreateEvent :!event OnHoldedItemActionEnded))
  (EventDispatchers|BindEventtoInteracted (Variables|Default|GetHoldedItem) (EventDispatchers|CreateEvent :!event ReleaseItem)))

(fn TryInteract
  (bind _camera (Variables|Character|GetCamera))
  (bind _returnvalue (Transformation|GetWorldLocation _camera))
  (bind _outhit (Collision|LineTraceByChannel _returnvalue (+ _returnvalue (* (Math|Vector|GetForwardVector _camera) (Variables|Default|GetLineTraceLength))) "TraceTypeQuery1" false 0 "None"))
  (Class|BPIInteractable|OnInteract(Message) (.HitActor (Collision|BreakHitResult _outhit)))
  (bind _asbp_holdable_item (Utilities|Casting|CastToBP_HoldableItem (.HitActor (Collision|BreakHitResult _outhit))))
  (if (not (Variables|/Game/TestTask/Blueprints/Environment/Interactables/HoldableItems/BP_HoldableItem.BP_HoldableItem_C|GetIsBusy _asbp_holdable_item))
    (CallFunction|PickUpItem _asbp_holdable_item)))

(fn ReleaseItem
  (Transformation|DetachFromActor (Variables|Default|GetHoldedItem) "KeepWorld" "KeepWorld" "KeepRelative")
  (Default|OnRelease (Variables|Default|GetHoldedItem))
  (Variables|Default|SetIsBusy false)
  (Default|CallItemReleased)
  (EventDispatchers|UnbindEventfromActionEnded (Variables|Default|GetHoldedItem) (EventDispatchers|CreateEvent :!event OnHoldedItemActionEnded))
  (EventDispatchers|UnbindEventfromInteracted (Variables|Default|GetHoldedItem) (EventDispatchers|CreateEvent :!event ReleaseItem)))

(fn OnHoldedItemActionEnded
  (Default|CallItemPickedUp (Variables|Default|GetHoldedItem)))