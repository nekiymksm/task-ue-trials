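; BP_ItemsCell is an environment cell that counts the holdable items of its designated kind currently inside its trigger.
; ItemsCount resets on BeginPlay, then rises on begin overlap and falls on end overlap for matching actors.
; IsRightItemKind casts to BP_HoldableItem and compares ItemKind from that actor's class defaults, rather than its instance value, against the cell's ItemsKind.
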(event OnComponentBeginOverlap(Trigger)
  (params (OverlappedComponent :type Primitive%20Component%20Object%20Reference) (OtherActor :type Actor%20Object%20Reference) (OtherComp :type Primitive%20Component%20Object%20Reference) (OtherBodyIndex :type Integer) (bFromSweep :type Boolean) (SweepResult :type Hit%20Result%20Structure%20%28by%20ref%29))
  (if (CallFunction|IsRightItemKind OtherActor)
    (Math|Integer|IncrementInt (Variables|Default|GetItemsCount))))

(event OnComponentEndOverlap(Trigger)
  (params (OverlappedComponent :type Primitive%20Component%20Object%20Reference) (OtherActor :type Actor%20Object%20Reference) (OtherComp :type Primitive%20Component%20Object%20Reference) (OtherBodyIndex :type Integer))
  (if (CallFunction|IsRightItemKind OtherActor)
    (Math|Integer|DecrementInt (Variables|Default|GetItemsCount))))

(event EventBeginPlay
  (Variables|Default|SetItemsCount 0))

(fn ConstructionScript)

(fn IsRightItemKind
  (params (Actor :type Actor%20Object%20Reference))
  (bind _asbp_holdable_item (Utilities|Casting|CastToBP_HoldableItem Actor))
  (return (Utilities|Enum|Equal(Enum) (.ItemKind (Utilities|GetClassDefaults (Utilities|GetClass _asbp_holdable_item))) (Variables|Default|GetItemsKind))))