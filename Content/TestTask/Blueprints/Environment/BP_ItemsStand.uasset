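; Item stand that holds a single item of a matching ItemKind and acts as a combine target.
; TryCombine checks kind and occupancy, fires the item's Interacted call, snaps it to SetPoint and sends it an OnInteract message.
; The stand then binds to that item's Interacted event, freeing itself when the item is picked up.
; GetItem exposes the held item, while GetKind always reports not busy.
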(event Custom|Event%20OnItemPickuped
  (EventDispatchers|UnbindEventfromInteracted (Variables|Default|GetCurrentItem) (delegate Custom|Event%20OnItemPickuped))
  (Variables|Default|SetIsBusy_0 false))

(event Custom|Event%20OnItemPlaced
  (EventDispatchers|BindEventtoInteracted (Variables|Default|GetCurrentItem) (delegate Custom|Event%20OnItemPickuped)))

(event EventTryCombine
  (params (OtherItem :type BP%20Holdable%20Item%20Object%20Reference))
  (if (CallFunction|CanPlace OtherItem)
    (Default|CallInteracted OtherItem)
    (CallFunction|Place OtherItem)))

(fn ConstructionScript)

(fn Place
  (params (Item :type BP%20Holdable%20Item%20Object%20Reference))
  (Variables|Default|SetCurrentItem Item)
  (Variables|Default|SetIsBusy_0 true)
  (Transformation|SetActorLocation (Variables|Default|GetCurrentItem) (Transformation|GetWorldLocation (Variables|Default|GetSetPoint)) false false)
  (Class|BPIInteractable|OnInteract(Message) (Variables|Default|GetCurrentItem))
  (CallFunction|EventonItemPlaced))

(fn CanPlace
  (params (Item :type BP%20Holdable%20Item%20Object%20Reference))
  (if (Utilities|Enum|Equal(Enum) (Variables|/Game/TestTask/Blueprints/Environment/Interactables/HoldableItems/BP_HoldableItem.BP_HoldableItem_C|GetItemKind Item) (Variables|Default|GetItemKind))
    (return (Math|Boolean|Equal(Boolean) (Variables|Default|GetIsBusy_0) false))
    (else
      (return false))))

(fn GetItem
  (if (Variables|Default|GetIsBusy_0)
    (return (Variables|Default|GetCurrentItem))))

(fn GetKind
  (return (Variables|Default|GetCombinableKind) false))