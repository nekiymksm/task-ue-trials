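; Interactable button that broadcasts an OnClick event with its Id when the player interacts with it.
; Interact is ignored while IsBusy is set; otherwise it fires the event, locks the button and plays the ButtonPush timeline.
; The timeline slides the View component along local Z by up to ZAxisSlideDistance and clears IsBusy when finished.
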(event EventInteract
  (if (not (Variables|Default|GetIsBusy))
    (Default|CallOnClick (Variables|Default|GetId))
    (Variables|Default|SetIsBusy true)
    (Components|Timeline|PlayfromStart (Variables|Default|GetButtonPush))))

(fn ConstructionScript)