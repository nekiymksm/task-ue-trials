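; Interactable liquid pump that broadcasts an interaction and, when its tumbler is opened, pours an animated stream of liquid.
; TryOpenTumbler plays the TurnTumbler timeline to rotate the tumbler, then TryReleaseLiquid runs the ReleaseLiquid timeline, scaling and moving LiquidNullPoint along Z.
; It announces the stream duration, derived from both timeline lengths, and sets a timer for it.
; OnWaterIntakeEnd closes the tumbler by reversing its timeline.
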(event EventOnInteract
  (Default|CallInteracted))

(fn ConstructionScript)

(fn OnWaterIntakeEnd
  (Variables|Default|SetIsTumblerOpen false)
  (Components|Timeline|ReversefromEnd (Variables|Default|GetTurnTumbler)))

(fn TryReleaseLiquid
  (if (Variables|Default|GetIsTumblerOpen)
    (LocalVariables|SetStreamDuration (- (Components|Timeline|GetTimelineLength (Variables|Default|GetReleaseLiquid)) (Components|Timeline|GetTimelineLength (Variables|Default|GetTurnTumbler))))
    (Utilities|Time|SetTimerbyEvent (EventDispatchers|CreateEvent :!event OnWaterIntakeEnd) (LocalVariables|GetStreamDuration))
    (Components|Timeline|PlayfromStart (Variables|Default|GetReleaseLiquid))
    (Variables|Default|SetLiquidStartPosition (Variables|/Script/Engine.SceneComponent|GetRelativeLocation (Variables|Default|GetLiquidNullPoint)))
    (Default|CallLiquidReleased (LocalVariables|GetStreamDuration))))

(fn SetLiquidStream
  (params (ZAxisScale :type Float%20%28single-precision%29) (ZAxisLocation :type Float%20%28single-precision%29))
  (bind _liquidnullpoint (Variables|Default|GetLiquidNullPoint))
  (Transformation|SetRelativeScale3D _liquidnullpoint (Math|Vector|MakeVector 1.0 1.0 ZAxisScale))
  (Transformation|SetRelativeLocation _liquidnullpoint (Math|Vector|MakeVector (.x (Variables|/Script/Engine.SceneComponent|GetRelativeLocation _liquidnullpoint)) 0.0 ZAxisLocation) false false))

(fn TryOpenTumbler
  (if (not (Variables|Default|GetIsTumblerOpen))
    (Variables|Default|SetIsTumblerOpen true)
    (Components|Timeline|PlayfromStart (Variables|Default|GetTurnTumbler))))