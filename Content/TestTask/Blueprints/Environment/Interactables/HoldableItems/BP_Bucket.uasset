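; Holdable bucket that stores a capped amount of liquid and can be filled, emptied or combined with another bucket.
; Timelines animate filling over a given duration and the tipping action that drains it, with the liquid level shown by Z-scaling LiquidNullPoint.
; Tick empties it instantly when the view's roll or pitch reaches 90 degrees.
; Combining pours the other bucket into this one up to capacity, leaving any remainder in the source.
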(event EventDoAction
  (if (not (Variables|Default|GetIsBusy))
    (Variables|Default|SetIsBusy true)
    (Components|Timeline|PlayfromStart (Variables|Default|GetDrainOut))))

(event EventTryCombine
  (params (OtherItem :type BP%20Holdable%20Item%20Object%20Reference))
  (if (Utilities|Enum|Equal(Enum) (Variables|/Game/TestTask/Blueprints/Environment/Interactables/HoldableItems/BP_HoldableItem.BP_HoldableItem_C|GetItemKind OtherItem) "NewEnumerator3")
    (CallFunction|Combine OtherItem)))

(event EventTick
  (params (DeltaSeconds :type Float%20%28single-precision%29))
  (bind _view (Variables|Default|GetView))
  (bind _returnvalue (Transformation|GetWorldRotation _view))
  (if (Variables|Default|GetIsNotEmpty)
    (if (or (>= (.roll _returnvalue) 9e+01) (>= (.pitch _returnvalue) 9e+01))
      (CallFunction|ToEmpty))))

(fn ConstructionScript
  (|CallParentFunction))

(fn Fill
  (params (Duration :type Float%20%28single-precision%29))
  (Components|Timeline|SetPlayRate (Variables|Default|GetLiquidIntake) (/ 1.0 Duration))
  (Components|Timeline|PlayfromStart (Variables|Default|GetLiquidIntake))
  (Variables|Default|SetIsBusy true))

(fn ToEmpty
  (Transformation|SetRelativeScale3D (Variables|Default|GetLiquidNullPoint) (Math|Vector|MakeVector 1.0 1.0 0.0))
  (Variables|Default|SetIsNotEmpty false)
  (Variables|Default|SetCurrentLiquidValue 0))

(fn GetValues
  (return (Variables|Default|GetCurrentLiquidValue) (Variables|Default|GetCapacity)))

(fn Transfuse
  (params (OtherBucket :type BP%20Bucket%20Object%20Reference))
  (bind _remainvalue (CallFunction|Take OtherBucket (Variables|Default|GetCurrentLiquidValue)))
  (Variables|Default|SetCurrentLiquidValue _remainvalue))

(fn Take
  (params (ReceivedValue :type Integer))
  (LocalVariables|SetCurrentReceivedValue ReceivedValue)
  (if (< (Variables|Default|GetCurrentLiquidValue) (Variables|Default|GetCapacity))
    (LocalVariables|SetRequiredValue (- (Variables|Default|GetCapacity) (Variables|Default|GetCurrentLiquidValue)))
    (if (< (LocalVariables|GetCurrentReceivedValue) (LocalVariables|GetRequiredValue))
      (Variables|Default|SetCurrentLiquidValue (+ (LocalVariables|GetCurrentReceivedValue) (Variables|Default|GetCurrentLiquidValue)))
      (return 0)
      (else
        (Variables|Default|SetCurrentLiquidValue (Variables|Default|GetCapacity))
        (return (- (LocalVariables|GetCurrentReceivedValue) (LocalVariables|GetRequiredValue)))))
    (else
      (return (LocalVariables|GetCurrentReceivedValue)))))

(fn SetLiquid
  (Transformation|SetRelativeScale3D (Variables|Default|GetLiquidNullPoint) (Math|Vector|MakeVector 1.0 1.0 (/ (Math|Conversions|ToFloat(Integer) (Variables|Default|GetCurrentLiquidValue)) (Math|Conversions|ToFloat(Integer) (Variables|Default|GetCapacity)))))
  (Variables|Default|SetIsNotEmpty (> (Variables|Default|GetCurrentLiquidValue) 0)))

(fn CanFill
  (return (< (Variables|Default|GetCurrentLiquidValue) (Variables|Default|GetCapacity))))

(fn Combine
  (params (Item :type BP%20Holdable%20Item%20Object%20Reference))
  (bind _asbp_bucket (Utilities|Casting|CastToBP_Bucket Item))
  (bind _output_get (LocalVariables|SetOtherBucket _asbp_bucket))
  (CallFunction|Transfuse _output_get self)
  (Default|CallActionEnded (LocalVariables|GetOtherBucket))
  (CallFunction|SetLiquid)
  (CallFunction|SetLiquid (LocalVariables|GetOtherBucket)))

(fn GetKind
  (return (Variables|Default|GetCombinableKind) (Variables|Default|GetIsBusy)))