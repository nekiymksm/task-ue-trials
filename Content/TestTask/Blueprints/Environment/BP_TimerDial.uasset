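; BP_TimerDial is a dial timer whose hand sweeps to show the progress of a countdown of a given duration.
; Start sets a one-shot timer and marks the dial active, while OnTimerEnd clears that active flag.
; It also scales the TurnArrow timeline's play rate by the inverse of the duration, driving a rotation lerp on AxisHand toward a full turn.
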(event Custom|Event%20Start
  (params (Duration :type Float%20%28single-precision%29))
  (Variables|Default|SetDuration Duration)
  (Utilities|FlowControl|Sequence
    (:then_0
      (Utilities|Time|SetTimerbyEvent (EventDispatchers|CreateEvent :!event OnTimerEnd) (Variables|Default|GetDuration))
      (Variables|Default|SetIsActive true))
    (:then_1
      (Components|Timeline|SetPlayRate (Variables|Default|GetTurnArrow) (/ 1.0 (Variables|Default|GetDuration)))
      (bind _float (Timeline|TurnArrow PlayFromStart)
        (:Update
          (Transformation|SetRelativeRotation (Variables|Default|GetAxisHand) (Math|Rotator|Lerp(Rotator) "0, 0, 0" "0,360.000000, 0" _float) false false))))))

(fn ConstructionScript)

(fn OnTimerEnd
  (Variables|Default|SetIsActive false))